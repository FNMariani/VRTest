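; BP_ChangeMaterialActor is an actor that toggles a material selection menu above itself, apparently for hand-based interaction.
; Toggling spawns a scaled-down, rotated BP_ChangeMaterialMenu actor, passing through which menu hand is active, or closes and destroys the existing one through its stored reference.
; Separate events show and hide a decal component as a selection indicator.
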(event `self.BP_CreateMaterialSelectionWidget`
  (params (bActiveMenuHandRight :type Boolean))
  (bind _returnvalue (`|SpawnActorFromClass` "/Game/Blueprints/BP_ChangeMaterialMenu.BP_ChangeMaterialMenu_C" (`KismetMathLibrary.MakeTransform` (+ (`self.K2_GetActorLocation`) (0.0 0.0 40.0)) (struct :`Yaw` -180.0) (0.1 0.1 0.1)) "Undefined" "MultiplyWithRoot" null bActiveMenuHandRight null))
  (set `self.ChangeMaterialMenuRef` _returnvalue))

(event `self.BP_RemoveMaterialSelectionWidget`
  (bind _changematerialmenuref (`self.ChangeMaterialMenuRef`))
  (`/Engine/EditorBlueprintResources/StandardMacros.IsValid` _changematerialmenuref
    (:`Is Valid`
      (`/Game/Blueprints/BP_ChangeMaterialMenu.CloseMenu` _changematerialmenuref)
      (`self.K2_DestroyActor` _changematerialmenuref)
      (set `self.ChangeMaterialMenuRef` null))))

(event `self.BP_ToggleMaterialSelectionWidget`
  (params (bActiveMenuHandRight :type Boolean))
  (`self.ChangeMaterialMenuRef`
    (:`then`
      (`self.BP_RemoveMaterialSelectionWidget`))
    (:`else`
      (`self.BP_CreateMaterialSelectionWidget` bActiveMenuHandRight))))

(event `self.BP_ShowSelectionDecal`
  (`SceneComponent.SetVisibility` (`self.DecalComponent`) true false))

(event `self.BP_HideSelectionDecal`
  (`SceneComponent.SetVisibility` (`self.DecalComponent`) false false))

(fn `UserConstructionScript`)